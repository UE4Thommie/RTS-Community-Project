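; MyCharacter is a selectable character that moves to given locations and shows a decal while selected.
; Selection calls Possess on the supplied controller and reveals the decal, which is hidden on spawn and deselection.
; DoAction sends its controller to the target with SimpleMoveToLocation.
; The construction script scales the decal from the mesh's bounding sphere radius, and BeginPlay prints the character type.
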(event EventBeginPlay
  (CallFunction|ToggleSelectionDecal true)
  (Development|PrintString (Utilities|String|Append "Spawned new player of type " (Utilities|String|EnumtoString (Variables|Default|GetCharacterType))) true false "(R=0.490991,G=1.000000,B=0.000000,A=1.000000)"))

(event EventDeselected
  (CallFunction|ToggleSelectionDecal true))

(event EventDoAction
  (params (Location :type Vector :default "0, 0, 0"))
  (AI|Navigation|SimpleMovetoLocation (Pawn|GetController) Location))

(event EventSelected
  (params (Controller :type Player%20Controller%20Object%20Reference))
  (Pawn|Possess Controller)
  (CallFunction|ToggleSelectionDecal false))

(fn ConstructionScript
  (Transformation|SetRelativeScale3D (Variables|Default|GetSelectionDecal) (Math|Conversions|ToVector(Float) (- (.SphereRadius (Collision|GetComponentBounds (Variables|Character|GetMesh))) 1e+02))))

(fn ToggleSelectionDecal
  (params (bHideDecal :type Boolean))
  (Development|SetHiddeninGame (Variables|Default|GetSelectionDecal) bHideDecal false))