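; RTS camera pawn that pans, rotates and zooms over the level.
; Each tick it moves the actor relative to the Sphere's facing, snaps the Sphere to a vertical trace hit to follow terrain height, and applies yaw input.
; Zoom input sets a clamped target distance that the spring arm interpolates toward, with curves scaling zoom step and pan speed by that distance.
; Pan and rotation are not scaled by delta time.
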(event EventBeginPlay)

(event EventActorBeginOverlap
  (params (OtherActor :type Actor%20Object%20Reference)))

(event EventTick
  (params (DeltaSeconds :type Float%20%28single-precision%29))
  (bind _returnvalue (Transformation|GetActorLocation))
  (Utilities|FlowControl|Sequence
    (:then_0
      (|DefaultMovement :!pinned true) ; Default Movement / Set actor location
    )
    (:then_1
      ;[1 1 1] Set Camera location
      (bind _outhit (Collision|LineTraceByChannel (+ _returnvalue "0, 0,500000.000000") (- _returnvalue "0, 0,500000.000000") "TraceTypeQuery3" false 0 "None"))
      (Transformation|SetWorldLocation (Variables|Default|GetSphere) (.Location (Collision|BreakHitResult _outhit)) false))
    (:then_2
      ;[1 1 1] Zooming
      (Variables|/Script/Engine.SpringArmComponent|SetTargetArmLength (Variables|Default|GetSpringArm) (Math|Interpolation|FInterpTo (Variables|/Script/Engine.SpringArmComponent|GetTargetArmLength (Variables|Default|GetSpringArm)) (Variables|Zoom|GetTargetDistance) DeltaSeconds 1e+01)))
    (:then_3
      ;[1 1 1] Rotation
      (Transformation|AddWorldRotation (Variables|Default|GetSphere) (Class|KismetMathLibrary|MakeRot 0.0 (* (Input|AxisValues|GetCameraRotation) (Variables|Rotation|GetRotationSpeed)) 0.0) false))))

(event Input|ActionEvents|InputActionCameraZoomIn
  ;[1 1 1] Zoom events
  (:Pressed
    (Variables|Zoom|SetTargetDistance (Math|Float|Clamp(Float) (- (Variables|Zoom|GetTargetDistance) (* (Math|Curves|GetFloatValue (Variables|Zoom|GetZoomCurve) (Variables|Zoom|GetTargetDistance)) (Variables|Zoom|GetZoomSpeed))) (Variables|Zoom|GetMinDistance) (Variables|Zoom|GetMaxDistance)))))

(event Input|ActionEvents|InputActionCameraZoomOut
  ;[1 1 1] Zoom events
  (:Pressed
    (Variables|Zoom|SetTargetDistance (Math|Float|Clamp(Float) (+ (Variables|Zoom|GetTargetDistance) (* (Math|Curves|GetFloatValue (Variables|Zoom|GetZoomCurve) (Variables|Zoom|GetTargetDistance)) (Variables|Zoom|GetZoomSpeed))) (Variables|Zoom|GetMinDistance) (Variables|Zoom|GetMaxDistance)))))

(fn ConstructionScript)