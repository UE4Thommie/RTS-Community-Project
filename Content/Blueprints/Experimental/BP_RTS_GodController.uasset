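; Experimental RTS god-style player controller that lets the player place houses with the mouse.
; On BeginPlay it spawns a construction manager at the world origin and keeps a reference to it.
; Each left-click traces under the cursor and queues a BP_House construction request at the hit location with that manager.
; A DoOnce, reset on button release, limits each press to one request.
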(event EventBeginPlay
  (bind _returnvalue (Game|SpawnActorfromClass "/Game/Blueprints/Experimental/Construction/BP_ConstructionManager.BP_ConstructionManager_C" (Math|Transform|MakeTransform "0, 0, 0") false 0))
  (Variables|Default|SetConstructionManager _returnvalue))

(event Input|ActionEvents|InputActionLMB
  (:Pressed
    (Utilities|FlowControl|DoOnce false :!label _label
      (:Completed
        (Default|QueueConstruction (Variables|Default|GetConstructionManager) (Utilities|Struct|MakeSTRUCT_ConstructionConf "/Game/Blueprints/Structures/BP_House.BP_House_C" (Math|Transform|MakeTransform (.Location (Collision|BreakHitResult (.HitResult (Game|Player|GetHitResultUnderCursorbyChannel "TraceTypeQuery3" true))))))))))
  (:Released
    (goto _label Reset)))

(fn ConstructionScript)