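; Construction manager that spawns proxy actors to stand in for buildings under construction, then swaps in the finished building.
; QueueConstruction picks a proxy class by building class, copies per-building stages and work hours onto multi-stage proxies, then initializes it with hardcoded workers.
; Parallel Queue and Proxies arrays pair each config with its proxy.
; On a proxy's completion event, it destroys that proxy, removes both entries and spawns the building at the stored transform.
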(event Custom|OnConstructionCompleted
  (params (Proxy :type BP%20Construction%20Proxy%20Object%20Reference))
  (CallFunction|FinishConstruction Proxy))

(fn ConstructionScript)

(fn QueueConstruction
  (params (Config :type STRUCT%20Construction%20Conf%20Structure))
  (bind (_buildingclass _transform) (Utilities|Struct|BreakSTRUCT_ConstructionConf Config))
  (bind _proxyclass (CallFunction|GetProxyClass _buildingclass))
  (bind _returnvalue (Game|SpawnActorfromClass _proxyclass _transform false))
  (bind _asbp_constructionproxy_c (Utilities|Casting|CastToBP_ConstructionProxy _returnvalue))
  (Utilities|FlowControl|Sequence
    (:then_0
      (CallFunction|ConfigureProxy _asbp_constructionproxy_c _buildingclass))
    (:then_1
      (EventDispatchers|BindEventtoConstructionCompleted _asbp_constructionproxy_c (EventDispatchers|CreateEvent self :!event Custom|OnConstructionCompleted))
      (Utilities|Array|Add (Variables|Default|GetProxies) _asbp_constructionproxy_c)
      (Utilities|Array|Add (Variables|Default|GetQueue) Config)
      (Default|Initialize _asbp_constructionproxy_c 0.0)
      (Default|SetWorkers _asbp_constructionproxy_c (Utilities|Array|MakeArray 1 2)))))

(fn FinishConstruction
  (params (Proxy :type BP%20Construction%20Proxy%20Object%20Reference))
  (LocalVariables|SetIndex (Utilities|Array|FindItem (Variables|Default|GetProxies) Proxy))
  (LocalVariables|SetConfig (Utilities|Array|Get(acopy) (Variables|Default|GetQueue) (LocalVariables|GetIndex)))
  (Actor|DestroyActor Proxy)
  (Utilities|Array|RemoveIndex (Variables|Default|GetQueue) (LocalVariables|GetIndex))
  (Utilities|Array|RemoveIndex (Variables|Default|GetProxies) (LocalVariables|GetIndex))
  (Game|SpawnActorfromClass (.BuildingClass (Utilities|Struct|BreakSTRUCT_ConstructionConf (LocalVariables|GetConfig))) (.Transform (Utilities|Struct|BreakSTRUCT_ConstructionConf (LocalVariables|GetConfig))) false))

(fn GetProxyClass
  (params (BuildingClass :type BP%20Building%20Master%20Class%20Reference))
  (bind _array_element (Utilities|Array|ForEachLoopwithBreak (Variables|Default|GetClassProxyList) :!label _label)
    (:LoopBody
      (if (== BuildingClass (.BuildingClass (Utilities|Struct|BreakSTRUCT_ProxyInf _array_element)))
        (LocalVariables|SetLocalProxyClass (.ProxyClass (Utilities|Struct|BreakSTRUCT_ProxyInf _array_element)))
        (goto _label Break)))
    (:Completed
      (return (LocalVariables|GetLocalProxyClass)))))

(fn ConfigureProxy
  (params (Proxy :type BP%20Construction%20Proxy%20Object%20Reference) (BuildingClass :type BP%20Building%20Master%20Class%20Reference))
  (Utilities|FlowControl|Sequence
    (:then_0
      (if (== (Utilities|GetClass Proxy) "/Game/Blueprints/Experimental/Construction/BP_MultiStageProxy.BP_MultiStageProxy_C")
        (CallFunction|SetMultiStageProxyConf Proxy BuildingClass)))))

(fn SetMultiStageProxyConf
  (params (Proxy :type BP%20Construction%20Proxy%20Object%20Reference) (BuildingClass :type BP%20Building%20Master%20Class%20Reference))
  (bind _asbp_multistageproxy_c (Utilities|Casting|CastToBP_MultiStageProxy Proxy))
  (bind _array_element (Utilities|Array|ForEachLoopwithBreak (Variables|Default|GetMultiStageProxyConf))
    (:LoopBody
      (if (== BuildingClass (.BuildingClass (Utilities|Struct|BreakSTRUCT_MultiStageProxyConf _array_element)))
        (Variables|/Game/Blueprints/Experimental/Construction/BP_MultiStageProxy.BP_MultiStageProxy_C|SetStages _asbp_multistageproxy_c (.Stages (Utilities|Struct|BreakSTRUCT_MultiStageProxyConf _array_element)))
        (Variables|/Game/Blueprints/Experimental/Construction/BP_ConstructionProxy.BP_ConstructionProxy_C|SetWorkHoursNeeded _asbp_multistageproxy_c (.WorkHoursNeeded (Utilities|Struct|BreakSTRUCT_MultiStageProxyConf _array_element)))))))