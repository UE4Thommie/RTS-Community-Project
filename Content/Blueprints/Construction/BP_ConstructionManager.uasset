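; BP_ConstructionManager manages building construction for a player, swapping placeholder proxies for finished buildings.
; QueueConstruction spawns a proxy from the config, records both in parallel arrays, sets its owner team state, initializes its work and assigns hardcoded workers.
; When the proxy's completion event fires, FinishConstruction finds its config by index, spawns and initializes the team-owned building, transfers any selection and destroys the proxy.
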(event Custom|BindConstructionCompleted
  (params (Proxy :type BP%20Construction%20Proxy%20Object%20Reference))
  (EventDispatchers|BindEventtoConstructionCompleted Proxy (delegate Custom|OnConstructionCompleted)))

(event Custom|OnConstructionCompleted
  (params (Proxy :type BP%20Construction%20Proxy%20Object%20Reference))
  (CallFunction|FinishConstruction Proxy))

(fn ConstructionScript)

(fn QueueConstruction
  (params (Config :type STRUCT%20Construction%20Conf%20Structure))
  (bind (_buildingclass _proxyclass _transform _workhoursneeded) (Utilities|Struct|BreakSTRUCT_ConstructionConf Config))
  (bind _returnvalue (Game|SpawnActorfromClass _proxyclass _transform false 0))
  (bind _asbp_construction_proxy (Utilities|Casting|CastToBP_ConstructionProxy _returnvalue))
  (CallFunction|BindConstructionCompleted _asbp_construction_proxy)
  (Utilities|Array|Add (Variables|Default|GetProxies) _asbp_construction_proxy)
  (Utilities|Array|Add (Variables|Default|GetQueue) Config)
  (Utilities|FlowControl|Sequence
    (:then_0
      (bind _asbp_rts_team_state (Utilities|Casting|CastToBP_RTS_TeamState (Variables|/Script/Engine.Controller|GetPlayerState (Variables|Default|GetOwnerPC))))
      (Variables|/Game/Blueprints/Construction/BP_ConstructionProxy.BP_ConstructionProxy_C|SetOwnerPlayerState _asbp_construction_proxy _asbp_rts_team_state))
    (:then_1
      (Default|Initialize _asbp_construction_proxy _workhoursneeded 0.0)
      (Default|SetWorkers _asbp_construction_proxy (Utilities|Array|MakeArray 1 2)))))

(fn FinishConstruction
  (params (Proxy :type BP%20Construction%20Proxy%20Object%20Reference))
  ;[1 1 1] We have a proxy as input. Using that find the index of construction conf that it reprecents
  (LocalVariables|SetIndex (Utilities|Array|FindItem (Variables|Default|GetProxies) Proxy))
  (LocalVariables|SetConfig (Utilities|Array|Get(acopy) (Variables|Default|GetQueue) (LocalVariables|GetIndex)))
  ;[1 1 1] Remove the proxy and copnf from both lists
  (Utilities|Array|RemoveIndex (Variables|Default|GetQueue) (LocalVariables|GetIndex))
  (Utilities|Array|RemoveIndex (Variables|Default|GetProxies) (LocalVariables|GetIndex))
  (bind _returnvalue (Game|SpawnActorfromClass (.BuildingClass (Utilities|Struct|BreakSTRUCT_ConstructionConf (LocalVariables|GetConfig))) (.Transform (Utilities|Struct|BreakSTRUCT_ConstructionConf (LocalVariables|GetConfig))) false 0))
  (bind _asbp_building_master (Utilities|Casting|CastToBP_Building_Master _returnvalue))
  (Utilities|FlowControl|Sequence
    (:then_0
      ;[1 1 1] Set team and initialize
      (if (!= (Variables|Default|GetOwnerPC) 0)
        (if (!= (Variables|/Script/Engine.Controller|GetPlayerState (Variables|Default|GetOwnerPC)) 0)
          (bind _asbp_rts_team_state (Utilities|Casting|CastToBP_RTS_TeamState (Variables|/Script/Engine.Controller|GetPlayerState (Variables|Default|GetOwnerPC))))
          (Default|SetPlayerState _asbp_building_master _asbp_rts_team_state)
          (Variables|/Game/Blueprints/BP_Building_Master.BP_Building_Master_C|SetOwnerPC _asbp_building_master (Variables|Default|GetOwnerPC))
          (Default|Initialize _asbp_building_master))))
    (:then_1
      ;[1 1 1] Select new building if proxy was selected
      (if (Variables|/Game/Blueprints/Construction/BP_ConstructionProxy.BP_ConstructionProxy_C|GetbIsSelected Proxy)
        (Default|SelectSingleUnit (Variables|Default|GetOwnerPC) _asbp_building_master)))
    (:then_2
      (Actor|DestroyActor Proxy))))